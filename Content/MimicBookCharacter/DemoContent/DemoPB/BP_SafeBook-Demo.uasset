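; Demo mimic safe-book actor that assembles a random look at BeginPlay and, when interactive, opens as a Character overlaps it.
; Construction slaves modular meshes to a master pose, groups them by part type (shell for containers, pages otherwise) and creates dynamic materials.
; BeginPlay shows one random mesh per group and randomizes cover materials, colors and custom cover textures.
; Overlaps drive AnimBP open flags; non-containers flip pages after staying open briefly.
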(event EventBeginPlay
  (bind _colors (Variables|Default|GetColors))
  (bind _covermaterialsdynamic (Variables|Default|GetCoverMaterialsDynamic))
  (bind _customcovertextures (Variables|Default|GetCustomCoverTextures))
  ;[1 1 1] Random setup
  (Utilities|FlowControl|Sequence
    (:then_0
      (bind _asabp_mimic_book_safe (Utilities|Casting|CastToABP_Mimic-book-safe (Components|SkeletalMesh|GetAnimInstance (Variables|Default|GetSkeletalMesh))))
      (Variables|Default|SetAnimBP_ref _asabp_mimic_book_safe))
    (:then_1
      (bind _output_get (Variables|Default|SetcanShowCover? false))
      (Rendering|SetVisibility (Variables|Default|GetCustom) _output_get false)
      (for _array_element (Variables|Default|GetAllParts)
        (for _array_element_2 (.MemberVar_1 (Utilities|Struct|BreakS_Book-Part _array_element))
          (Rendering|SetVisibility _array_element_2 false false)
          (bind _output_get_2 (Variables|Default|SetRandomIndex (Math|Random|RandomIntegerinRange 0 (- (Utilities|Array|Length (.MemberVar_1 (Utilities|Struct|BreakS_Book-Part _array_element))) 1)))))
        (Rendering|SetVisibility (Utilities|Array|Get(acopy) (.MemberVar_1 (Utilities|Struct|BreakS_Book-Part _array_element)) _output_get_2) true false)
        (Rendering|SetBoundsScale (Utilities|Array|Get(acopy) (.MemberVar_1 (Utilities|Struct|BreakS_Book-Part _array_element)) _output_get_2) 1.0)
        (if (and (Utilities|Enum|Equal(Enum) (.MemberVar_0 (Utilities|Struct|BreakS_Book-Part _array_element)) "NewEnumerator3") (or (not (Utilities|IsValid (Variables|/Script/Engine.SkinnedMeshComponent|GetSkeletalMesh (Utilities|Array|Get(acopy) (.MemberVar_1 (Utilities|Struct|BreakS_Book-Part _array_element)) _output_get_2)))) (== (Utilities|Array|Get(acopy) (.MemberVar_1 (Utilities|Struct|BreakS_Book-Part _array_element)) _output_get_2) (Variables|/Script/Engine.SkinnedMeshComponent|GetSkeletalMesh (Variables|Default|GetCustom)))))
          (Variables|Default|SetcanShowCover? true)
          (if (Variables|Default|GetcanShowCover?)
            (Rendering|SetVisibility (Variables|Default|GetCustom) true false)
            (bind _output_get_3 (Variables|Default|SetRandomTextureIndex (Math|Random|RandomIntegerinRange 0 (- (Utilities|Array|Length _customcovertextures) 1))))
            (for (_array_element_3 _array_index) (Variables|Default|GetDMI_CustomCover)
              (Rendering|Material|SetTextureParameterValue _array_element_3 "MainTex" (Utilities|Array|Get(acopy) _customcovertextures _output_get_3))
              (Rendering|Material|SetMaterial (Variables|Default|GetCustom) _array_index _array_element_3))))))
    (:then_2
      ;[1 1 1] Random cover material
      (Utilities|IsValid (Utilities|Array|Get(acopy) _covermaterialsdynamic (stale _output_get_4))
        (:Is%20Valid
          (bind _output_get_4 (Variables|Default|SetRandomIndex (Math|Random|RandomIntegerinRange 0 (- (Utilities|Array|Length _covermaterialsdynamic) 1))))
          (CallFunction|SetMaterialbyPartType "NewEnumerator1" (Utilities|Array|Get(acopy) _covermaterialsdynamic _output_get_4))
          (CallFunction|SetMaterialbyPartType "NewEnumerator5" (Utilities|Array|Get(acopy) _covermaterialsdynamic _output_get_4))
          (if (== _output_get_4 3)
            (bind _output_get_5 (Variables|Default|SetRandomColorIndex (Math|Random|RandomIntegerinRange 0 (- (Utilities|Array|Length _colors) 1))))
            (CallFunction|SetColor _output_get_5 _colors (Utilities|Array|Get(acopy) _covermaterialsdynamic _output_get_4))
            (else
              (CallFunction|SetColor -1 _colors (Utilities|Array|Get(acopy) _covermaterialsdynamic _output_get_4)))))))
    (:then_3
      (if (Variables|Default|GetIsContainer)
        (Rendering|SetVisibility (Variables|Default|GetSkeletalMesh) false false)))))

(event Collision|EventActorBeginOverlap
  (params (OtherActor :type Actor%20Object%20Reference))
  (bind _animbp_ref (Variables|Default|GetAnimBP_ref))
  (if (Variables|Default|GetIsInteractive)
    (Utilities|IsValid _animbp_ref
      (:Is%20Valid
        (Utilities|Casting|CastToCharacterClass (Utilities|GetClass OtherActor))
        (Variables|/Game/MimicBookCharacter/Animations/ABP_Mimic-book-safe.ABP_Mimic-book-safe_C|SetisOpen _animbp_ref true)))))

(event Collision|EventActorEndOverlap
  (params (OtherActor :type Actor%20Object%20Reference))
  (bind _animbp_ref (Variables|Default|GetAnimBP_ref))
  (if (Variables|Default|GetIsInteractive)
    (Utilities|IsValid _animbp_ref
      (:Is%20Valid
        (Variables|/Game/MimicBookCharacter/Animations/ABP_Mimic-book-safe.ABP_Mimic-book-safe_C|SetisOpen _animbp_ref false)
        (Variables|/Game/MimicBookCharacter/Animations/ABP_Mimic-book-safe.ABP_Mimic-book-safe_C|SetisFlipPages _animbp_ref false)
        (Variables|Default|SetOpenTime 0.0)))))

(event EventTick
  (params (DeltaSeconds :type Float%20%28single-precision%29))
  (bind _animbp_ref (Variables|Default|GetAnimBP_ref))
  (if (Variables|Default|GetIsInteractive)
    (if (not (Variables|Default|GetIsContainer))
      (Utilities|IsValid _animbp_ref
        (:Is%20Valid
          (if (Variables|/Game/MimicBookCharacter/Animations/ABP_Mimic-book-safe.ABP_Mimic-book-safe_C|GetisOpen _animbp_ref)
            (bind _output_get (Variables|Default|SetOpenTime (+ (Variables|Default|GetOpenTime) DeltaSeconds)))
            (if (> _output_get 1.0)
              (Variables|/Game/MimicBookCharacter/Animations/ABP_Mimic-book-safe.ABP_Mimic-book-safe_C|SetisFlipPages _animbp_ref true))))))))

(fn ConstructionScript
  (bind _skeletalmesh (Variables|Default|GetSkeletalMesh))
  (Utilities|FlowControl|Sequence
    (:then_0
      (for _array_element (Actor|GetComponentsByClass "/Script/Engine.SkeletalMeshComponent")
        (if (not (== _array_element _skeletalmesh))
          (Class|SkinnedMeshComponent|SetMasterPoseComponent _array_element _skeletalmesh false)
          (Variables|/Script/Engine.SceneComponent|SetbUseAttachParentBound _array_element true)
          (bind _partsarrayout (CallFunction|AddParts (Variables|Default|GetAllParts) "NewEnumerator3" (Utilities|Array|MakeArray (Variables|Default|GetDeco-1) (Variables|Default|GetDeco-2) (Variables|Default|GetDeco-3) (Variables|Default|GetDeco-4) (Variables|Default|GetDeco-5) (Variables|Default|GetDeco-6) (Variables|Default|GetNothing) (Variables|Default|GetNothing))))
          (bind _partsarrayout_2 (CallFunction|AddParts _partsarrayout "NewEnumerator4" (Utilities|Array|MakeArray (Variables|Default|GetHinges-2) (Variables|Default|GetHinges-3) (Variables|Default|GetHinges-1) (Variables|Default|GetNothing))))
          (bind _partsarrayout_3 (CallFunction|AddParts _partsarrayout_2 "NewEnumerator7" (Utilities|Array|MakeArray (Variables|Default|GetCorners-1) (Variables|Default|GetCorners-2) (Variables|Default|GetCorners-3) (Variables|Default|GetCorners-4) (Variables|Default|GetNothing))))
          (bind _partsarrayout_4 (CallFunction|AddParts _partsarrayout_3 "NewEnumerator6" (Utilities|Array|MakeArray (Variables|Default|GetConnector-1) (Variables|Default|GetConnector-2) (Variables|Default|GetConnector-3) (Variables|Default|GetNothing))))
          (bind _partsarrayout_5 (CallFunction|AddParts _partsarrayout_4 "NewEnumerator5" (Utilities|Array|MakeArray (Variables|Default|GetRoot-1) (Variables|Default|GetRoot-2) (Variables|Default|GetRoot-3) (Variables|Default|GetNothing))))
          (bind _partsarrayout_6 (CallFunction|AddParts _partsarrayout_5 "NewEnumerator1" (Utilities|Array|MakeArray (Variables|Default|GetCover))))
          (if (Variables|Default|GetIsContainer)
            (Rendering|SetVisibility (Variables|Default|GetSkeletalMesh) false false)
            (bind _partsarrayout_7 (CallFunction|AddParts _partsarrayout_6 "NewEnumerator8" (Utilities|Array|MakeArray (Variables|Default|GetShell))))
            (Variables|Default|SetAllParts _partsarrayout_7)
            (else
              (bind _partsarrayout_8 (CallFunction|AddParts _partsarrayout_6 "NewEnumerator2" (Utilities|Array|MakeArray (Variables|Default|GetPages))))
              (Variables|Default|SetAllParts _partsarrayout_8))))))
    (:then_1
      (for _array_element_2 (Variables|Default|GetCoverMaterials)
        (Utilities|IsValid _array_element_2
          (:Is%20Valid
            (bind _returnvalue (Rendering|Material|CreateDynamicMaterialInstance _array_element_2 "None" :!class /Script/Engine.KismetMaterialLibrary))
            (Utilities|Array|AddUnique (Variables|Default|GetCoverMaterialsDynamic) _returnvalue))))
      (for _array_element_3 (Rendering|Material|GetMaterials (Variables|Default|GetCustom))
        (bind _returnvalue_2 (Rendering|Material|CreateDynamicMaterialInstance _array_element_3 "None" :!class /Script/Engine.KismetMaterialLibrary))
        (Utilities|Array|AddUnique (Variables|Default|GetDMI_CustomCover) _returnvalue_2)))))

(fn AddParts
  (params (PartsArrayIn :type Array%20of%20S%20Book-Part%20Structures) (PartsType :type E_Book-parts%20Enum :default "NewEnumerator0") (PartSMComponents :type Array%20of%20Skeletal%20Mesh%20Component%20Object%20References))
  (Utilities|Array|AddUnique PartsArrayIn (Utilities|Struct|MakeS_Book-Part PartsType PartSMComponents))
  (return PartsArrayIn))

(fn SetColor
  (params (ColorIndex :type Integer) (Colors :type Array%20of%20Color%20Structures) (DMaterial :type Material%20Instance%20Dynamic%20Object%20Reference))
  (bind _returnvalue (Utilities|Array|Length Colors))
  (if (or (< ColorIndex 0) (>= 0 _returnvalue))
    (Rendering|Material|SetVectorParameterValue DMaterial "Color" (Math|Conversions|ToLinearColor(Color) (Utilities|Array|Get(acopy) Colors (Math|Random|RandomIntegerinRange 0 (- _returnvalue 1)))) :!class /Script/Engine.MaterialInstanceDynamic)
    (Rendering|Material|SetScalarParameterValue 0 (Utilities|Name|MakeLiteralName "Metalic") 0.0 :!class /Script/Engine.KismetMaterialLibrary)
    (Rendering|Material|SetScalarParameterValue 0 (Utilities|Name|MakeLiteralName "Roughness") 2.0 :!class /Script/Engine.KismetMaterialLibrary)
    (else
      (Rendering|Material|SetVectorParameterValue DMaterial "Color" (Math|Conversions|ToLinearColor(Color) (Utilities|Array|Get(acopy) Colors ColorIndex)) :!class /Script/Engine.MaterialInstanceDynamic))))

(fn SetMaterialbyPartType
  (params (PartsType :type E_Book-parts%20Enum :default "NewEnumerator0") (DMInstance :type Material%20Instance%20Dynamic%20Object%20Reference))
  (for _array_element (Variables|Default|GetAllParts)
    (if (Utilities|Enum|Equal(Enum) (.MemberVar_0 (Utilities|Struct|BreakS_Book-Part _array_element)) PartsType)
      (for _array_element_2 (.MemberVar_1 (Utilities|Struct|BreakS_Book-Part _array_element))
        (Rendering|Material|SetMaterial _array_element_2 0 DMInstance)))))