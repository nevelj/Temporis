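; Child actor that customizes and randomizes its parent goblin's body, face, skin, eyes and warpaint.
; Construction finds the "GoblinMesh"-tagged mesh, optionally randomizes it, then applies the CharacterData and MaterialData maps.
; CharacterData keys name morph targets, except head size, sent to the AnimBP by interface; warpaint sets scalar parameters on a dynamic skin material.
; Both maps save to a slot, optionally named after the parent, with optional auto-load on BeginPlay.
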(event Custom|Event_Apply_Warpaint
  ;[1 0 0.7747 1 40] Material Update / Application
  (|UpdatetheDynamicMaterialaccordingtotheWarpaintVariables))

(event Custom|Event_RandomEyeMaterial
  (bind _eyematerialoptions (Variables|CharacterCreator|GetEyeMaterialOptions))
  ;[1 0.02059 0.9723 1 40] Material Randomization
  (Utilities|Map|Add (Variables|CharacterCreator|GetMaterialData) "Eye_Type" (Math|Random|RandomIntegerinRange 0 (Utilities|Array|Length _eyematerialoptions)))
  (Rendering|Material|SetMaterial (Variables|OperationalVariables|GetSkeletalMesh) 0 (Utilities|Array|Get(acopy) _eyematerialoptions (.Value (Utilities|Map|Find (Variables|CharacterCreator|GetMaterialData) "Eye_Type"))))
  (CallFunction|EventApplyEyeMaterial))

(event Custom|Event_Apply_SkinType
  ;[1 0 0.7747 1 40] Material Update / Application
  (Rendering|Material|SetMaterial (Variables|OperationalVariables|GetSkeletalMesh) 1 (Utilities|Array|Get(acopy) (Variables|CharacterCreator|GetSkinMaterialOptions) (.Value (Utilities|Map|Find (Variables|CharacterCreator|GetMaterialData) "Skin_Type"))))
  (CallFunction|MakeSkinMaterialDynamic)
  (CallFunction|EventApplyWarpaint) ; Since we changed the skin material, we must reapply warpaints settings to it
)

(event Custom|Event_ApplyAllValues
  ;[1 0.8719 0 1 40] Apply All Values
  (CallFunction|EventApplyMorphValuesandHeadSize)
  (CallFunction|EventApplyWarpaint)
  (CallFunction|EventApplySkinType)
  (CallFunction|EventApplyEyeMaterial))

(event Custom|Event_Randomize_SkinType
  ;[1 0.02059 0.9723 1 40] Material Randomization
  (Utilities|Map|Add (Variables|CharacterCreator|GetMaterialData) "Skin_Type" (Math|Random|RandomIntegerinRange 0 (Utilities|Array|Length (Variables|CharacterCreator|GetSkinMaterialOptions))))
  (CallFunction|EventApplySkinType))

(event Custom|Event_ApplyMorphValues_andHeadSize
  ;[1 0 0 1 40] Apply Variables to Skeletal Mesh (Morph Targets & Head Bone)
  (if (Variables|OperationalVariables|GetCanAccessSkeletalMesh)
    (|ApplyVariablestoMorphTargets)))

(event Custom|Event_Randomize_Warpaint
  ;[1 0.02059 0.9723 1 40] Material Randomization
  (|RandomizeWarpaintVariablesandCall"UpdateWarpaint"))

(event Custom|Randomize
  ;[1 0.9973 0 1 40] Randomize Values for Procedural Generation
  (if (Variables|OperationalVariables|GetCanAccessSkeletalMesh)
    (|SetRandomVariables) ; Change the values inside this node to \nalter the outcomes \nof procedural generation
    (CallFunction|EventApplyMorphValuesandHeadSize)))

(event Custom|Event_ApplyEyeMaterial
  ;[1 0 0.7747 1 40] Material Update / Application
  (Rendering|Material|SetMaterial (Variables|OperationalVariables|GetSkeletalMesh) 0 (Utilities|Array|Get(acopy) (Variables|CharacterCreator|GetEyeMaterialOptions) (.Value (Utilities|Map|Find (Variables|CharacterCreator|GetMaterialData) "Eye_Type")))))

(event EventBeginPlay
  ;[1 0 0.8697 1 40] Saving and Loading
  ;;[1 0 0.8697 1 40] Auto-Load (Optional)
  (if (Variables|SavingAndLoading|GetAuto-Load%20Values)
    (CallFunction|LoadCharacterCreatorValues)))

(fn ConstructionScript
  (Variables|OperationalVariables|SetSkeletalMesh (Utilities|Array|Get(acopy) (Actor|GetComponentsbyTag (Actor|GetParentActor) "/Script/Engine.SkeletalMeshComponent" "GoblinMesh")))
  (Utilities|IsValid (Variables|OperationalVariables|GetSkeletalMesh)
    (:Is%20Valid
      (Variables|OperationalVariables|SetCanAccessSkeletalMesh true)
      (CallFunction|MakeSkinMaterialDynamic)
      ;[1 1 1] Initial Randomization
      (if (Variables|CharacterRandomization|GetRandomize%20Morphs%20OnStart)
        (CallFunction|Randomize))
      (if (Variables|CharacterRandomization|GetRandomize%20Skin%20on%20Start)
        (CallFunction|EventRandomizeSkinType))
      (if (Variables|CharacterRandomization|GetRandomize%20Warpaint%20on%20Start)
        (CallFunction|EventRandomizeWarpaint))
      (if (Variables|CharacterRandomization|GetRandomize%20Eye%20Type%20on%20Start)
        (CallFunction|EventRandomEyeMaterial))
      (CallFunction|EventApplyMorphValuesandHeadSize)
      (CallFunction|EventApplySkinType)
      (CallFunction|EventApplyEyeMaterial)
      (CallFunction|EventApplyWarpaint))))

(fn MakeSkinMaterialDynamic
  (bind _returnvalue (Rendering|Material|CreateDynamicMaterialInstance (Utilities|Array|Get(acopy) (Rendering|Material|GetMaterials (Variables|OperationalVariables|GetSkeletalMesh)) 1) "None" "None" :!class /Script/Engine.KismetMaterialLibrary)) ; Create a Dynamic Material Instance for the Goblin Skin for altering Warpaint
  (Variables|OperationalVariables|SetDynamicMaterial_GoblinSkin _returnvalue)
  (Rendering|Material|SetMaterial (Variables|OperationalVariables|GetSkeletalMesh) 1 (Variables|OperationalVariables|GetDynamicMaterial_GoblinSkin)) ; Apply the Dynamic Material instance to the goblin
)

(fn ApplyMorphTargetfromCharacterDataVariable
  (params (MorphTargetName :type Name))
  (bind _returnvalue (Utilities|String|ToString(Name) MorphTargetName))
  (bind _characterdata (Variables|CharacterCreator|GetCharacterData))
  (bind (_value _returnvalue_2) (Utilities|Map|Find _characterdata _returnvalue))
  (if _returnvalue_2
    (Components|SkeletalMesh|SetMorphTarget (Components|SkeletalMesh|GetAnimInstance (Variables|OperationalVariables|GetSkeletalMesh)) MorphTargetName _value)
    (else
      (Development|PrintString "Morph Target Name Invalid - Please check BP_CharacterCreator for correct naming" true true "(R=1.000000,G=0.040715,B=0.000000,A=1.000000)" 1e+01))))

(fn EditValue
  (params (Key :type String) (Value :type Float%20%28double-precision%29%20%28by%20ref%29))
  (Utilities|Map|Add (Variables|CharacterCreator|GetCharacterData) Key Value))

(fn SaveCharacterCreatorValues
  (bind _returnvalue (Actor|GetParentActor))
  (bind _savegame_slot_name (Variables|SavingAndLoading|GetSaveGame%20Slot%20Name))
  (bind _savegame_slotname_is_objectname (Variables|SavingAndLoading|GetSaveGame%20SlotName%20is%20ObjectName))
  (bind _returnvalue_2 (Utilities|GetDisplayName _returnvalue))
  (bind _returnvalue_3 (Utilities|String|SelectString _returnvalue_2 _savegame_slot_name _savegame_slotname_is_objectname))
  (bind _returnvalue_4 (SaveGame|DoesSaveGameExist _returnvalue_3))
  (if _returnvalue_4
    (bind _returnvalue_5 (SaveGame|LoadGamefromSlot _returnvalue_3)) ; Load Existing SaveGame Object so we can Overwrite its Data
    (bind _asbp_character_creator_goblin_save_game (Utilities|Casting|CastToBP_CharacterCreator_Goblin_SaveGame _returnvalue_5))
    (Variables|SavingandLoading|SetSaveGame%20Object _asbp_character_creator_goblin_save_game)
    (else
      (bind _returnvalue_6 (SaveGame|CreateSaveGameObject "/Game/Goblin/Blueprints/CharacterCreator/BP_CharacterCreator_Goblin_SaveGame.BP_CharacterCreator_Goblin_SaveGame_C")) ; create save game object
      (Variables|SavingandLoading|SetSaveGame%20Object _returnvalue_6)))
  (Variables|/Game/Goblin/Blueprints/CharacterCreator/BP_CharacterCreator_Goblin_SaveGame.BP_CharacterCreator_Goblin_SaveGame_C|SetCharacterData (Variables|SavingandLoading|GetSaveGame%20Object) (Variables|CharacterCreator|GetCharacterData))
  (Variables|/Game/Goblin/Blueprints/CharacterCreator/BP_CharacterCreator_Goblin_SaveGame.BP_CharacterCreator_Goblin_SaveGame_C|SetMaterialData (Variables|SavingandLoading|GetSaveGame%20Object) (Variables|CharacterCreator|GetMaterialData))
  (SaveGame|SaveGametoSlot (Variables|SavingandLoading|GetSaveGame%20Object) _returnvalue_3))

(fn LoadCharacterCreatorValues
  (bind _returnvalue (Actor|GetParentActor))
  (bind _savegame_slot_name (Variables|SavingAndLoading|GetSaveGame%20Slot%20Name))
  (bind _savegame_slotname_is_objectname (Variables|SavingAndLoading|GetSaveGame%20SlotName%20is%20ObjectName))
  (bind _returnvalue_2 (Utilities|GetDisplayName _returnvalue))
  (bind _returnvalue_3 (Utilities|String|SelectString _returnvalue_2 _savegame_slot_name _savegame_slotname_is_objectname))
  (bind _returnvalue_4 (SaveGame|DoesSaveGameExist _returnvalue_3))
  (if _returnvalue_4
    (bind _returnvalue_5 (SaveGame|LoadGamefromSlot _returnvalue_3)) ; Load Existing SaveGame Object
    (bind _asbp_character_creator_goblin_save_game (Utilities|Casting|CastToBP_CharacterCreator_Goblin_SaveGame _returnvalue_5))
    (bind _output_get (Variables|SavingandLoading|SetSaveGame%20Object _asbp_character_creator_goblin_save_game))
    (Variables|CharacterCreator|SetCharacterData (Variables|/Game/Goblin/Blueprints/CharacterCreator/BP_CharacterCreator_Goblin_SaveGame.BP_CharacterCreator_Goblin_SaveGame_C|GetCharacterData _output_get))
    (Variables|CharacterCreator|SetMaterialData (Variables|/Game/Goblin/Blueprints/CharacterCreator/BP_CharacterCreator_Goblin_SaveGame.BP_CharacterCreator_Goblin_SaveGame_C|GetMaterialData _output_get))
    (CallFunction|EventApplyAllValues)
    (elif (Variables|SavingAndLoading|GetAuto-Load%20Values)
      (|CreateSaveGamesinceAuto-LoadistrueandaSaveGamedoesntexistyet _returnvalue_3)
      (elif (Variables|Default|GetDebug)
        (Development|PrintString "An attempt at Loading Character Creator values has been made - but there is not current SaveGame holding these values! Check BP_CharacterCreator_Goblin and its SaveGame Slot Name for errors" true true "(R=1.000000,G=0.000000,B=0.038652,A=1.000000)" 1e+01)))))