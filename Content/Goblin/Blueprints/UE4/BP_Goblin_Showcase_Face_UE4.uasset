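; Goblin showcase Blueprint that displays the character with a selectable Stone Age weapon.
; The construction script switches on WeaponType to show a club, spear or warhammer mesh component.
; It attaches the chosen weapon to the hand_lSocket on the Mesh with KeepWorld rules, so the weapon keeps its world transform.
; The event graph holds only disabled placeholder events, so it adds no runtime logic.
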(event Collision|EventActorBeginOverlap
  (params (OtherActor :type Actor%20Object%20Reference)))

(event EventTick
  (params (DeltaSeconds :type Float%20%28single-precision%29)))

(fn ConstructionScript
  (bind _sm_stoneage_warhammer (Variables|Default|GetSM_StoneAge_Warhammer))
  (switch int (Variables|Default|GetWeaponType)
    (:1
      (Rendering|SetVisibility (Variables|Default|GetSM_StoneAge_Club) true false)
      (Transformation|AttachComponentToComponent (Variables|Default|GetSM_StoneAge_Club) (Variables|Default|GetMesh) "hand_lSocket" "KeepWorld" "KeepWorld" "KeepWorld" true))
    (:2
      (Rendering|SetVisibility (Variables|Default|GetSM_StoneAge_Spear) true false)
      (Transformation|AttachComponentToComponent (Variables|Default|GetSM_StoneAge_Spear) (Variables|Default|GetMesh) "hand_lSocket" "KeepWorld" "KeepWorld" "KeepWorld" true))
    (:3
      (Rendering|SetVisibility _sm_stoneage_warhammer true false)
      (Transformation|AttachComponentToComponent _sm_stoneage_warhammer (Variables|Default|GetMesh) "hand_lSocket" "KeepWorld" "KeepWorld" "KeepWorld" true))))