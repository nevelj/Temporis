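; Goblin showcase actor that displays a configurable skeletal mesh with an optional stone age weapon and links to a Goblin character creator child actor.
; The construction script applies the chosen mesh, then uses the weapon type to reveal a club, spear or warhammer and attach it to the left-hand socket, keeping world transform.
; Save and Load events cast the child actor and forward to its functions that save or load character creator values.
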(event Custom|Event_Save
  (bind _asbp_character_creator_goblin (Utilities|Casting|CastToBP_CharacterCreator_Goblin (Variables|/Script/Engine.ChildActorComponent|GetChildActor (Variables|Default|GetBP_CharacterCreator_Goblin))))
  (Default|SaveCharacterCreatorValues _asbp_character_creator_goblin))

(event Custom|Event_Load
  (bind _asbp_character_creator_goblin (Utilities|Casting|CastToBP_CharacterCreator_Goblin (Variables|/Script/Engine.ChildActorComponent|GetChildActor (Variables|Default|GetBP_CharacterCreator_Goblin))))
  (Default|LoadCharacterCreatorValues _asbp_character_creator_goblin))

(fn ConstructionScript
  (bind _sm_stoneage_warhammer (Variables|Default|GetSM_StoneAge_Warhammer))
  (Components|SkeletalMesh|SetSkeletalMeshAsset (Variables|Default|GetMesh) (Variables|Default|GetSkeletalMesh))
  (switch int (Variables|Default|GetWeaponType)
    (:1
      (Rendering|SetVisibility (Variables|Default|GetSM_StoneAge_Club) true false)
      (Transformation|AttachComponentToComponent (Variables|Default|GetSM_StoneAge_Club) (Variables|Default|GetMesh) "hand_lSocket" "KeepWorld" "KeepWorld" "KeepWorld" true))
    (:2
      (Rendering|SetVisibility (Variables|Default|GetSM_StoneAge_Spear) true false)
      (Transformation|AttachComponentToComponent (Variables|Default|GetSM_StoneAge_Spear) (Variables|Default|GetMesh) "hand_lSocket" "KeepWorld" "KeepWorld" "KeepWorld" true))
    (:3
      (Rendering|SetVisibility _sm_stoneage_warhammer true false)
      (Transformation|AttachComponentToComponent _sm_stoneage_warhammer (Variables|Default|GetMesh) "hand_lSocket" "KeepWorld" "KeepWorld" "KeepWorld" true))))